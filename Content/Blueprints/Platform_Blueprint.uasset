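; Player-controlled platform pawn that possesses itself on BeginPlay and slides its Cube around a bounded horizontal area.
; Each Tick, Move offsets the Cube by the input vector, capped at unit length to prevent faster diagonals, scaled by Speed and delta time.
; It clamps world X/Y within ±BoundaryWidth and writes that as relative location with Z zero.
; The DebugSpawn input calls Spawn on the level's Spawner_Blueprint.
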(event `self.ReceiveBeginPlay`
  (bind _returnvalue (`GameplayStatics.GetPlayerController` 0))
  (`Controller.Possess` _returnvalue self)
  (`self.EnableInput` _returnvalue))

(event `self.ReceiveTick`
  (params (DeltaSeconds :type "Float (single-precision)"))
  (`self.Move` DeltaSeconds))

(event `InputAction|DebugSpawn`
  (params (Key :type "Key Structure"))
  (:`Pressed`
    (bind _returnvalue (`GameplayStatics.GetActorOfClass` "/Game/Blueprints/Spawner_Blueprint.Spawner_Blueprint_C"))
    (`/Game/Blueprints/Spawner_Blueprint.Spawn` _returnvalue)))

(fn `Get Movement Vector`
  (returns (`Movement Vector` :type "Vector Structure"))
  (bind _returnvalue (`KismetMathLibrary.MakeVector` (`self.GetInputAxisValue`) (`self.GetInputAxisValue`)))
  (bind _returnvalue_2 (`KismetMathLibrary.Normal` _returnvalue))
  (if (> (`KismetMathLibrary.VSize` _returnvalue) (`KismetMathLibrary.VSize` _returnvalue_2))
    (return _returnvalue_2)
    (else
      (return _returnvalue))))

(fn `Move`
  (params (`Delta Seconds` :type "Float (double-precision)"))
  (bind _cube (`self.Cube`))
  (bind _boundary_width (`self.Boundary Width`))
  (bind _returnvalue (* -1 _boundary_width))
  (bind _movement_vector (`self.Get Movement Vector`))
  (`SceneComponent.K2_AddLocalOffset` _cube (* _movement_vector (* `Delta Seconds` (`self.Speed`))) false false)
  (`SceneComponent.K2_SetRelativeLocation` _cube (`KismetMathLibrary.MakeVector` (`KismetMathLibrary.FClamp` (.x (`SceneComponent.K2_GetComponentLocation` _cube)) _returnvalue _boundary_width) (`KismetMathLibrary.FClamp` (.y (`SceneComponent.K2_GetComponentLocation` _cube)) _returnvalue _boundary_width)) false false))

(fn `UserConstructionScript`)