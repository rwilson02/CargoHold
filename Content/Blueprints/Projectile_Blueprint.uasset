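; Projectile actor that reacts to sphere collisions with physics-simulated objects.
; On hit, it applies an impulse at its own location, derived from its velocity, then destroys itself; hits on non-simulating components do nothing.
; The velocity multiplier is a zero vector, so the impulse has no effect as written.
; The remaining spawn, move, timeline and component-creation nodes are disconnected leftovers, and the construction script is empty.
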(event `InputAction|DebugSpawn`
  (params (Key :type "Key Structure"))
  ;[1 1 1] Put in level BP
)

(event `self.Sphere_Collision.OnComponentHit`
  (params (HitComponent :type "PrimitiveComponent Object Reference") (OtherActor :type "Actor Object Reference") (OtherComp :type "PrimitiveComponent Object Reference") (NormalImpulse :type "Vector Structure") (Hit :type "HitResult Structure (by ref)"))
  (if (`SceneComponent.IsSimulatingPhysics` OtherComp "None")
    (`PrimitiveComponent.AddImpulseAtLocation` OtherComp (* (`self.GetVelocity`) (0.0 0.0 0.0)) (`self.K2_GetActorLocation`) "None")
    (`self.K2_DestroyActor`)))

(fn `UserConstructionScript`)