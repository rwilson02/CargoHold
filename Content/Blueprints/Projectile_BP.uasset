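; Projectile_BP is a projectile actor that reacts to hitting physics objects.
; On Hit, if the other component simulates physics, it applies a velocity-based impulse at its location, scaled by zero, and destroys itself; other hits leave it alive.
; A DebugSpawn input spawns another Projectile_BP at the actor's own transform.
; The construction script is empty, and a few leftover nodes never run.
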(event `InputAction|DebugSpawn`
  (params (Key :type "Key Structure"))
  (:`Pressed`
    (`|SpawnActorFromClass` "Projectile_BP_C" (`KismetMathLibrary.MakeTransform` (+ (.location (`self.GetTransform`)) (0.0 0.0 0.0)) (.rotation (`self.GetTransform`)) (.scale (`self.GetTransform`))) "Undefined" "OverrideRootScale" null null)))

(event `self.ReceiveHit`
  (params (MyComp :type "PrimitiveComponent Object Reference") (Other :type "Actor Object Reference") (OtherComp :type "PrimitiveComponent Object Reference") (bSelfMoved :type Boolean) (HitLocation :type "Vector Structure") (HitNormal :type "Vector Structure") (NormalImpulse :type "Vector Structure") (Hit :type "HitResult Structure (by ref)"))
  (if (`SceneComponent.IsSimulatingPhysics` OtherComp "None")
    (`PrimitiveComponent.AddImpulseAtLocation` OtherComp (* (`self.GetVelocity`) 0.0) (`self.K2_GetActorLocation`) "None")
    (`self.K2_DestroyActor`)))

(fn `UserConstructionScript`)