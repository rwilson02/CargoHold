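; Spawner actor that repeatedly fires ProjectileRandomLocal_BP projectiles from its Projectile component.
; Tick runs into a short Delay, which throttles spawning to a fixed interval.
; Each spawn takes the component's world location and a rotation rebuilt from its forward vector.
; Unconnected leftover nodes for spawning Projectile_BP1 and Projectile_BP2 and toggling component tick never execute.
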(event `self.ReceiveBeginPlay`)

(event `self.ReceiveTick`
  (params (DeltaSeconds :type "Float (single-precision)"))
  (bind _projectile (`self.Projectile`))
  (`KismetSystemLibrary.Delay` 0.2)
  (`|SpawnActorFromClass` "/Game/Blueprints/RandomizedProjectiles/ProjectileRandomLocal_BP.ProjectileRandomLocal_BP_C" (`KismetMathLibrary.MakeTransform` (`SceneComponent.K2_GetComponentLocation` _projectile) (`KismetMathLibrary.Conv_VectorToRotator` (`KismetMathLibrary.Conv_RotatorToVector` (`SceneComponent.K2_GetComponentRotation` _projectile)))) "Undefined" "OverrideRootScale" null (0.0 0.0 0.0) (0.0 0.0 0.0) null))

(fn `UserConstructionScript`)