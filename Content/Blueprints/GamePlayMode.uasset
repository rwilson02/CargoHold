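; GamePlayMode is a game mode Blueprint that runs the gameplay HUD, score and game-over screen.
; BeginPlay creates the gameplay HUD widget and adds it to the viewport.
; While GameOver is false, Tick adds time-scaled points from ScorePerSec and ScoreMultiplier to Score, rounding the result every frame.
; Once GameOver is true, scoring stops and a DoOnce adds the game-over widget to the viewport a single time.
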(event `self.ReceiveBeginPlay`
  (bind _returnvalue (`|CreateWidget` "/Game/UI_Widgets/GameplayHUD_WidgetBP.GameplayHUD_WidgetBP_C"))
  (`UserWidget.AddToViewport` _returnvalue 0))

(event `self.ReceiveTick`
  (params (DeltaSeconds :type "Float (single-precision)"))
  (if (`self.GameOver`)
    (`/Engine/EditorBlueprintResources/StandardMacros.DoOnce` false
      (:`Completed`
        (bind _returnvalue (`|CreateWidget` "/Game/UI_Widgets/GameplayOverHUD_WidgetBP.GameplayOverHUD_WidgetBP_C"))
        (`UserWidget.AddToViewport` _returnvalue 0)))
    (else
      (set `self.Score` (`KismetMathLibrary.Round` (+ (`KismetMathLibrary.Conv_IntToDouble` (`self.Score`)) (* DeltaSeconds (`self.ScoreMultiplier`) (`self.ScorePerSec`))))))))

(fn `UserConstructionScript`)