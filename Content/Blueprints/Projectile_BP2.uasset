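; Projectile actor that travels between two configurable relative locations using an InterpToMovement component rather than launched physics.
; The construction script builds the two control points from its location variables and sets the travel duration.
; On hit, it applies an impulse at its location to physics-simulating components, but the velocity multiplier is zero, so the push has no effect.
; Leftover destroy and mesh-description nodes are unconnected and never run.
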(event `self.ReceiveHit`
  (params (MyComp :type "PrimitiveComponent Object Reference") (Other :type "Actor Object Reference") (OtherComp :type "PrimitiveComponent Object Reference") (bSelfMoved :type Boolean) (HitLocation :type "Vector Structure") (HitNormal :type "Vector Structure") (NormalImpulse :type "Vector Structure") (Hit :type "HitResult Structure (by ref)"))
  ;[1 1 1] From Projectiles Project
  (if (`SceneComponent.IsSimulatingPhysics` OtherComp "None")
    (`PrimitiveComponent.AddImpulseAtLocation` OtherComp (* (`self.GetVelocity`) 0.0) (`self.K2_GetActorLocation`) "None")))

(fn `UserConstructionScript`
  (bind _interptomovement (`self.InterpToMovement`))
  ;[1 1 1] Projectile Movement
  (set `InterpToMovementComponent.ControlPoints` (`|MakeArray` (make `InterpControlPoint` (`self.Location 1`)) (make `InterpControlPoint` (`self.Locaton 2`))) _interptomovement)
  (set `InterpToMovementComponent.Duration` (`self.Durration`) _interptomovement))